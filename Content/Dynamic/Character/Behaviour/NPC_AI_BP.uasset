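; AI controller for guard NPCs that runs the GuardBehaviour tree on the PatrolData blackboard.
; Perception updates ignore actors tagged "Enemy"; any other sensed actor is stored in the "Enemy" blackboard key, which is cleared when sensing is lost.
; The same events switch IsAiming and IsShooting together on the controlled FP_TPCharacterBP, on while sensing and off at start or on loss.
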(event `self.ReceiveBeginPlay`
  (`self.UseBlackboard` "/Game/Dynamic/Character/Behaviour/PatrolData.PatrolData")
  (`self.RunBehaviorTree` "/Game/Dynamic/Character/Behaviour/GuardBehaviour.GuardBehaviour")
  (bind _asfp_tpcharacter_bp (cast `/Game/Dynamic/Character/Behaviour/FP_TPCharacterBP` (`self.K2_GetPawn` self)))
  (bind _output_get (set `/Game/Dynamic/Character/Behaviour/FP_TPCharacterBP.IsAiming` false _asfp_tpcharacter_bp))
  (set `/Game/Dynamic/Character/Behaviour/FP_TPCharacterBP.isShooting` _output_get _asfp_tpcharacter_bp))

(event `self.AIPerception.OnTargetPerceptionUpdated`
  (params (Actor :type "Actor Object Reference") (Stimulus :type "AIStimulus Structure"))
  (bind _returnvalue (`self.K2_GetPawn` self))
  (if (`self.ActorHasTag` Actor "Enemy")
    _
    (elif (`.bSuccessfullySensed` (break `AIStimulus` Stimulus))
      (`BlackboardComponent.SetValueAsObject` (`AIBlueprintHelperLibrary.GetBlackboard` self) (`KismetStringLibrary.Conv_StringToName` "Enemy") Actor)
      (bind _asfp_tpcharacter_bp (cast `/Game/Dynamic/Character/Behaviour/FP_TPCharacterBP` _returnvalue))
      (bind _output_get (set `/Game/Dynamic/Character/Behaviour/FP_TPCharacterBP.IsAiming` true _asfp_tpcharacter_bp))
      (set `/Game/Dynamic/Character/Behaviour/FP_TPCharacterBP.isShooting` _output_get _asfp_tpcharacter_bp)
      (else
        (`BlackboardComponent.ClearValue` (`AIBlueprintHelperLibrary.GetBlackboard` self) (`KismetStringLibrary.Conv_StringToName` "Enemy"))
        (bind _asfp_tpcharacter_bp_2 (cast `/Game/Dynamic/Character/Behaviour/FP_TPCharacterBP` _returnvalue))
        (bind _output_get_2 (set `/Game/Dynamic/Character/Behaviour/FP_TPCharacterBP.IsAiming` false _asfp_tpcharacter_bp_2))
        (set `/Game/Dynamic/Character/Behaviour/FP_TPCharacterBP.isShooting` _output_get_2 _asfp_tpcharacter_bp_2)))))

(fn `UserConstructionScript`)