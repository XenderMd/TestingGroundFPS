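; Game mode for an infinite terrain game that spawns the starting tiles and tracks a "Tiles Conquered" score.
; On BeginPlay it fills a bounds volume pool, spawns the first few tiles, then initializes and prints the score.
; SpawnTiles chains each BP_Tile onto the previous one's attach location and hands it the shared NavMeshBoundsVolume pool.
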(event `self.ReceiveBeginPlay`
  (`self.PopulateBoundsVolumePool`)
  (for _ (range 3)
    (`self.SpawnTiles`))
  (`|ExecutionSequence`
    (:`then_0`
      (`self.InitializeScore`))
    (:`then_1`
      (`self.DisplayScore`))))

(fn `DisplayScore`
  (bind _returnvalue (`self.GetScore`))
  (`KismetSystemLibrary.PrintString` (`KismetStringLibrary.Concat_StrStr` "Tiles Conquered: " (`KismetStringLibrary.Conv_IntToString` _returnvalue))))

(fn `SpawnTiles`
  (bind _returnvalue (`|SpawnActorFromClass` "/Game/Dynamic/Terrain/BP_Tile.BP_Tile_C" (`self.NextSpawnTransform`) "Undefined" "OverrideRootScale" null null))
  (bind _attach_transform (`/Game/Dynamic/Terrain/BP_Tile.Get Attach Location` _returnvalue))
  (set `self.NextSpawnTransform` _attach_transform)
  (`Tile_CPP.SetActorPool` _returnvalue (`self.NavMeshBoundsVolumePool`)))

(fn `UserConstructionScript`)