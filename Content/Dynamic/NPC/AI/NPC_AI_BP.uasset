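; NPC_AI_BP is an AI controller for guard NPCs that feeds perception results into a behavior tree.
; On BeginPlay it sets up the PatrolData blackboard and runs the GuardBehaviour tree.
; Perception updates for actors without the "Enemy" tag set the blackboard's Enemy key to that actor when sensed, and clear it when sensing fails.
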(event `self.ReceiveBeginPlay`
  (`self.UseBlackboard` "/Game/Dynamic/NPC/Behaviour/PatrolData.PatrolData")
  (`self.RunBehaviorTree` "/Game/Dynamic/NPC/Behaviour/GuardBehaviour.GuardBehaviour"))

(event `self.AIPerception.OnTargetPerceptionUpdated`
  (params (Actor :type "Actor Object Reference") (Stimulus :type "AIStimulus Structure"))
  (if (`self.ActorHasTag` Actor "Enemy")
    _
    (elif (`.bSuccessfullySensed` (break `AIStimulus` Stimulus))
      (`BlackboardComponent.SetValueAsObject` (`AIBlueprintHelperLibrary.GetBlackboard` self) (`KismetStringLibrary.Conv_StringToName` "Enemy") Actor)
      (else
        (`BlackboardComponent.ClearValue` (`AIBlueprintHelperLibrary.GetBlackboard` self) (`KismetStringLibrary.Conv_StringToName` "Enemy"))))))

(fn `UserConstructionScript`)