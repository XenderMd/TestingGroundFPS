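; Behavior tree task that selects the next patrol waypoint for an AI-controlled NPC.
; It reads the PatrolPoints array from the cast pawn, then writes the point at the Blackboard Index to the Waypoint key.
; It then increments Index modulo the array length so the route loops, and finishes successfully.
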(event `self.ReceiveExecuteAI`
  (params (OwnerController :type "AIController Object Reference") (ControlledPawn :type "Pawn Object Reference"))
  (`self.Get Patrol Points` ControlledPawn)
  (`self.Set Next Waypoint`)
  (`self.CycleIndex`)
  (`self.FinishExecute` true))

(fn `CycleIndex`
  (bind _result (`/Engine/EditorBlueprintResources/StandardMacros.IncrementInt` (`BTFunctionLibrary.GetBlackboardValueAsInt` (`self.Index`)))
    (:`  `
      (`BTFunctionLibrary.SetBlackboardValueAsInt` (`self.Index`) (mod _result (`KismetArrayLibrary.Array_Length` (`self.Patrol Points`)))))))

(fn `Get Patrol Points`
  (params (Object :type "Object Object Reference"))
  (bind _aspatrolling_guard (cast `` Object))
  (set `self.Patrol Points` (`/Game/Dynamic/NPC/Behaviour/ChoseNextWaypoint_BP.Patrol Points` _aspatrolling_guard)))

(fn `Set Next Waypoint`
  (`BTFunctionLibrary.SetBlackboardValueAsObject` (`self.Waypoint`) (`|GetArrayItem` (`self.Patrol Points`) (`BTFunctionLibrary.GetBlackboardValueAsInt` (`self.Index`)))))