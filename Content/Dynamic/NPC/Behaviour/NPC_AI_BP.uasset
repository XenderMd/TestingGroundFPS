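; AI controller for a patrolling guard NPC that reacts to actors it perceives.
; On BeginPlay it sets up the PatrolData blackboard and runs the GuardBehaviour tree.
; Perception updates ignore actors tagged "Enemy"; sensing any other actor stores it in the "Enemy" blackboard key and turns on the guard's aiming and shooting flags.
; Losing the stimulus clears the key and both flags.
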(event `self.ReceiveBeginPlay`
  (`self.UseBlackboard` "/Game/Dynamic/NPC/Behaviour/PatrolData.PatrolData")
  (`self.RunBehaviorTree` "/Game/Dynamic/NPC/Behaviour/GuardBehaviour.GuardBehaviour"))

(event `self.AIPerception.OnTargetPerceptionUpdated`
  (params (Actor :type "Actor Object Reference") (Stimulus :type "AIStimulus Structure"))
  (bind _returnvalue (`self.K2_GetPawn` self))
  (if (`self.ActorHasTag` Actor "Enemy")
    _
    (elif (`.bSuccessfullySensed` (break `AIStimulus` Stimulus))
      (`BlackboardComponent.SetValueAsObject` (`AIBlueprintHelperLibrary.GetBlackboard` self) (`KismetStringLibrary.Conv_StringToName` "Enemy") Actor)
      (bind _aspatrolling_guard (cast `/Game/Dynamic/NPC/Behaviour/PatrollingGuard` _returnvalue))
      (bind _output_get (set `/Game/Dynamic/NPC/Behaviour/PatrollingGuard.IsAiming` true _aspatrolling_guard))
      (set `/Game/Dynamic/NPC/Behaviour/PatrollingGuard.isShooting` _output_get _aspatrolling_guard)
      (else
        (`BlackboardComponent.ClearValue` (`AIBlueprintHelperLibrary.GetBlackboard` self) (`KismetStringLibrary.Conv_StringToName` "Enemy"))
        (bind _aspatrolling_guard_2 (cast `/Game/Dynamic/NPC/Behaviour/PatrollingGuard` _returnvalue))
        (bind _output_get_2 (set `/Game/Dynamic/NPC/Behaviour/PatrollingGuard.IsAiming` false _aspatrolling_guard_2))
        (set `/Game/Dynamic/NPC/Behaviour/PatrollingGuard.isShooting` _output_get_2 _aspatrolling_guard_2)))))

(fn `UserConstructionScript`)