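; BP_Tile is a terrain tile for an infinite-terrain game mode, exposing an arrow transform as its attach point.
; On BeginPlay it unlocks two barriers (green) and scatters random containers, sandbags, canisters and rocks through PlaceActors.
; Player overlap with the floor volume locks Barrier2 (red, blocking).
; When the player leaves the wall volume, it asks the game mode to spawn tiles, locks Barrier1 and calls DestroyActor.
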(event `self.ReceiveBeginPlay`
  (`self.Unlock Wall` (`self.Barrier1`))
  (`self.Unlock Wall` (`self.Barrier2`))
  (`self.PlaceActors` "/Game/Dynamic/Terrain/Props/BP_Container.BP_Container_C" 500.0 1 3)
  (`self.PlaceActors` "/Game/Dynamic/Terrain/Props/BP_SandbagsWall.BP_SandbagsWall_C" 300.0 1 3)
  (`self.PlaceActors` "/Game/Dynamic/Terrain/Props/BP_Canister.BP_Canister_C" 50.0 1 20)
  (`self.PlaceActors` "/Game/Dynamic/Terrain/Props/BP_Rock5.BP_Rock5_C" 300.0 1 5)
  (`self.PlaceActors` "/Game/Dynamic/Terrain/Props/BP_Rock1.BP_Rock1_C" 150.0 1 10)
  (`self.PlaceActors` "/Game/Dynamic/Terrain/Props/BP_Rock17.BP_Rock17_C" 300.0 1 5))

(event `self.Locking Volume Wall.OnComponentBeginOverlap`
  (params (OverlappedComponent :type "PrimitiveComponent Object Reference") (OtherActor :type "Actor Object Reference") (OtherComp :type "PrimitiveComponent Object Reference") (OtherBodyIndex :type Integer) (bFromSweep :type Boolean) (SweepResult :type "HitResult Structure (by ref)")))

(event `self.Locking Volume Wall.OnComponentEndOverlap`
  (params (OverlappedComponent :type "PrimitiveComponent Object Reference") (OtherActor :type "Actor Object Reference") (OtherComp :type "PrimitiveComponent Object Reference") (OtherBodyIndex :type Integer))
  (`self.Is Player Actor` OtherActor)
  (bind _asinfinite_terrain_game_mode (cast `/Game/Dynamic/GameModes/InfiniteTerrainGameMode` (`GameplayStatics.GetGameMode`)))
  (`/Game/Dynamic/GameModes/InfiniteTerrainGameMode.SpawnTiles` _asinfinite_terrain_game_mode)
  (`self.Lock Wall` (`self.Barrier1`))
  (`self.K2_DestroyActor`))

(event `self.LockingVolume Floor.OnComponentBeginOverlap`
  (params (OverlappedComponent :type "PrimitiveComponent Object Reference") (OtherActor :type "Actor Object Reference") (OtherComp :type "PrimitiveComponent Object Reference") (OtherBodyIndex :type Integer) (bFromSweep :type Boolean) (SweepResult :type "HitResult Structure (by ref)"))
  (`self.Is Player Actor` OtherActor)
  (`self.Lock Wall` (`self.Barrier2`)))

(event `self.ReceiveTick`
  (params (DeltaSeconds :type "Float (single-precision)")))

(fn `Get Attach Location`
  (returns (`Attach Transform` :type "Transform Structure"))
  (return (`SceneComponent.K2_GetComponentToWorld` (`self.Arrow`))))

(fn `Lock Wall`
  (params (Barrier :type "PrimitiveComponent Object Reference"))
  (`PrimitiveComponent.SetCollisionEnabled` Barrier "QueryAndPhysics")
  (`PrimitiveComponent.SetMaterial` Barrier 0 "/Game/Dynamic/Terrain/MI_Barrier_Red.MI_Barrier_Red"))

(fn `Unlock Wall`
  (params (Barrier :type "PrimitiveComponent Object Reference"))
  (`PrimitiveComponent.SetCollisionEnabled` Barrier "PhysicsOnly")
  (`PrimitiveComponent.SetMaterial` Barrier 0 "/Game/Dynamic/Terrain/MI_Barrier_Green.MI_Barrier_Green"))

(fn `UserConstructionScript`)